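; GM_Industry drives endless enemy spawning for the Industry game mode, begun by its StartGame event.
; StartGame clears all widgets and plays the TLIndustry timeline, which acts as the spawn timer by restarting after each spawn.
; Each finish spawns a random RefEnemy class at a random BP_SpawnPoint location and sets its movement to Walking.
; The spawn point pick uses RandomInteger on the last index, so the final point is never chosen.
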(event Custom|StartGame
  (bind _refenemy (Variables|Default|GetRefEnemy))
  (Viewport|RemoveAllWidgets)
  (Timeline|TLIndustry Play
    (:Finished
      (bind _outactors (Actor|GetAllActorsOfClass "/Game/Blueprints/Enemies/BP_SpawnPoint.BP_SpawnPoint_C"))
      (bind _returnvalue (Game|SpawnActorfromClass (Utilities|Array|Get(acopy) _refenemy (Math|Random|RandomIntegerinRange 0 (Utilities|Array|LastIndex _refenemy))) (Math|Transform|MakeTransform (Transformation|GetActorLocation (Utilities|Array|Get(acopy) _outactors (Math|Random|RandomInteger (Utilities|Array|LastIndex _outactors)))) "0, 0, 0" "1,1,1") "Undefined" 0 0))
      (Pawn|Components|CharacterMovement|SetMovementMode (Variables|/Script/Engine.Character|GetCharacterMovement _returnvalue) "MOVE_Walking" 0)
      (Timeline|TLIndustry PlayFromStart))))

(fn ConstructionScript)