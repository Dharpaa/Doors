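; Player character Blueprint that shows an on-screen interaction prompt and supports jumping.
; On BeginPlay it creates BP_PlayerWidget, stores the reference and adds it to the viewport.
; OnInteractableFound and OnInteractableLost show and hide that widget's InteractText, with no detection logic in this graph.
; The Jump input press calls Jump directly.
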(event EventBeginPlay
  (bind _returnvalue (UserInterface|CreateWidget "/Game/Blueprints/Widget/BP_PlayerWidget.BP_PlayerWidget_C"))
  (bind _output_get (Variables|Default|SetWidgetRef _returnvalue))
  (UserInterface|Viewport|AddtoViewport _output_get 0))

(event EventOnInteractableFound
  (Widget|SetVisibility (Variables|/Game/Blueprints/Widget/BP_PlayerWidget.BP_PlayerWidget_C|GetInteractText (Variables|Default|GetWidgetRef)) "Visible"))

(event EventOnInteractableLost
  (Widget|SetVisibility (Variables|/Game/Blueprints/Widget/BP_PlayerWidget.BP_PlayerWidget_C|GetInteractText (Variables|Default|GetWidgetRef)) "Hidden"))

(event Input|ActionEvents|InputActionJump
  (params (Key :type Key%20Structure :default "None"))
  (:Pressed
    (Character|Jump)))

(fn ConstructionScript)