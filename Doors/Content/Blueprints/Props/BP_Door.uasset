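; BP_Door is a door prop that both the player and DoorsEnemy characters can operate.
; A tap calls Interact with player-specific open and close durations.
; A DoorsEnemy entering the Box calls InteractByAI with enemy durations, unless IALeaveDoorOpen is set and the door is already open.
; Icon and montage getters return empty, IsInteractable returns false, and the door motion logic lives outside these graphs.
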(event OnComponentBeginOverlap(Box)
  (params (OverlappedComponent :type Primitive%20Component%20Object%20Reference) (OtherActor :type Actor%20Object%20Reference) (OtherComp :type Primitive%20Component%20Object%20Reference) (OtherBodyIndex :type Integer) (bFromSweep :type Boolean) (SweepResult :type Hit%20Result%20Structure%20%28by%20ref%29))
  (bind _asdoors_enemy (Utilities|Casting|CastToDoorsEnemy OtherActor))
  (if (not (and (Variables|Default|GetIALeaveDoorOpen) (Class|PropDoor|IsOpened)))
    (Class|PropDoor|InteractbyAI _asdoors_enemy (Variables|Default|GetEnemyOpenDuration) (Variables|Default|GetEnemyCloseDuration))))

(event EventOnTap
  (Class|PropDoor|Interact (Variables|Default|GetPlayerOpenDuration) (Variables|Default|GetPlayerCloseDuration)))

(fn ConstructionScript)

(fn GetCancelIcon
  (return 0))

(fn GetTapIcon
  (return 0))

(fn InteractAnimMontage
  (return 0))

(fn IsInteractable
  (return false))